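; BP_Hammer is a hammer actor with pick-up and drop events, built around a component named Spline.
; PickUp turns off physics on Spline, snaps it to the given parent's location while keeping world rotation and scale, then writes spline point 0's world location back as a point location.
; Drop re-enables physics and detaches the actor, keeping its world transform.
; An unconnected cast to BP_VRHand never runs.
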(event `/Game/Blueprints/BPI_PickupActor.PickUp`
  (params (AttachTo :type "SceneComponent Object Reference"))
  (bind _spline (`self.Spline`))
  (`PrimitiveComponent.SetSimulatePhysics` (`self.Spline`) false)
  (`SceneComponent.K2_AttachToComponent` (`self.Spline`) AttachTo "None" "SnapToTarget" "KeepWorld" "KeepWorld" false)
  (`SplineComponent.SetLocationAtSplinePoint` _spline 0 (`SplineComponent.GetLocationAtSplinePoint` _spline 0 "World") "World" false))

(event `/Game/Blueprints/BPI_PickupActor.Drop`
  (`PrimitiveComponent.SetSimulatePhysics` (`self.Spline`) true)
  (`self.K2_DetachFromActor` "KeepWorld" "KeepWorld" "KeepWorld"))

(fn `UserConstructionScript`)